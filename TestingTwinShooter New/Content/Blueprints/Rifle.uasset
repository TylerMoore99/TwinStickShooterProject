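; Rifle weapon Blueprint that fires automatically while the trigger is held, spawning Projectile_Rifle actors with an attached gunshot sound.
; PullTrigger passes a DoOnce to fire immediately and start a looping timer paced by RoundsPerSecond; ReleaseTrigger clears both.
; Each Rifle call decrements Ammo; reaching zero skips the shot and, if reserve remains, refills to MagSize after a delay, deducting a hardcoded amount from ReserveAmmo.
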(event `PullTrigger`
  (`/Engine/EditorBlueprintResources/StandardMacros.DoOnce` false :!label _label
    (:`Completed`
      (if (not (== (`self.Ammo`) 0))
        (`self.Rifle`)
        (`KismetSystemLibrary.K2_SetTimer` null "Rifle" (/ 1.0 (`self.Rounds Per Second`)) true)))))

(event `ReleaseTrigger`
  (`KismetSystemLibrary.K2_ClearTimer` null "Rifle")
  (goto _label :!via `Reset`))

(event `Rifle`
  ;[1 1 1] Firing Bullets
  (set `self.Ammo` (- (`self.Ammo`) 1))
  (if (== (`self.Ammo`) 0)
    (if (not (== (`self.ReserveAmmo`) 0))
      (`KismetSystemLibrary.Delay` 2.0)
      (set `self.Ammo` (`self.MagSize`))
      (set `self.ReserveAmmo` (- (`self.ReserveAmmo`) 30)))
    (else
      (`|SpawnActorFromClass` "/Game/Blueprints/Projectile_Rifle.Projectile_Rifle_C" (`SceneComponent.K2_GetComponentToWorld` (`self.ProjectilerSpawnPoint`)) "Undefined" "OverrideRootScale" null null)
      (`GameplayStatics.SpawnSoundAttached` "/Game/Sounds/Rifle.Rifle" (`self.GunMesh`) "None" (0.0 0.0 0.0) (struct) "KeepRelativeOffset" false 1.0 1.0 0.0 null null))))

(fn `UserConstructionScript`
  (`parent.UserConstructionScript`))