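; Zombie enemy for a twin-stick game that repeatedly damages an overlapping BaseCharacter on a timer set by its attack rate.
; AffectHealth plays a sound, updates health and emits blood whose particle collisions spawn randomized splatter decals.
; On death it detaches its controller, disables damage and some collision, awards kill and score through TwinStickMode, drops a random power-up, then destroys itself after a delay.
; Construction tints the mesh through a dynamic material.
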(event `self.ReceiveBeginPlay`)

(event `/Game/Blueprints/IDamageable.AffectHealth`
  (params (Delta :type "Float (single-precision)"))
  (bind _powerups (`self.Powerups`))
  (bind _capsulecomponent (`self.CapsuleComponent`))
  ;[1 1 1] Damage To Enemy & Value of Score
  (`GameplayStatics.SpawnSoundAttached` "/Game/Sounds/SC_Zombie.SC_Zombie" (`self.Mesh`) "None" (0.0 0.0 0.0) (struct) "KeepRelativeOffset" false 1.0 1.0 0.0 null null)
  (`self.Calculate Health` Delta)
  ;[1 1 1] Blood Splat
  (bind _returnvalue (`GameplayStatics.SpawnEmitterAttached` "/Game/Blueprints/Blood_Splat/Blood_Splat_P.Blood_Splat_P" (`self.Mesh`) "None" (0.0 0.0 150.0)))
  (add `ParticleSystemComponent.OnParticleCollide` _returnvalue (delegate `OnCollideEvent`))
  (`KismetSystemLibrary.PrintString` (`KismetStringLibrary.Conv_DoubleToString` (`self.Health`)))
  (if (`self.IsDead`)
    (`self.DetachFromControllerPendingDestroy`)
    (`ActorComponent.K2_DestroyComponent` (`self.DamageVolume`))
    (`PrimitiveComponent.SetCollisionResponseToChannel` _capsulecomponent "ECC_WorldDynamic" "ECR_Ignore")
    (`PrimitiveComponent.SetCollisionResponseToChannel` _capsulecomponent "ECC_Pawn" "ECR_Ignore")
    (bind _astwin_stick_mode (cast `/Game/Blueprints/TwinStickMode` (`GameplayStatics.GetGameMode`)))
    (`/Game/Blueprints/TwinStickMode.IncrementKills` _astwin_stick_mode 1)
    (`/Game/Blueprints/TwinStickMode.IncrementScore` _astwin_stick_mode 100)
    (`|SpawnActorFromClass` (`|GetArrayItem` _powerups (`KismetMathLibrary.RandomIntegerInRange` 0 (- (`KismetArrayLibrary.Array_Length` _powerups) 1))) (`KismetMathLibrary.Conv_VectorToTransform` (`self.K2_GetActorLocation`)) "Undefined" "OverrideRootScale" null null)
    (`KismetSystemLibrary.Delay` 5.0)
    (`self.K2_DestroyActor`)))

(event `self.ReceiveActorBeginOverlap`
  (params (OtherActor :type "Actor Object Reference"))
  ;[1 1 1] Damage To Player
  (bind _asbase_character (cast `/Game/Blueprints/BaseCharacter` OtherActor))
  (set `self.Player` _asbase_character)
  (`KismetSystemLibrary.K2_SetTimer` null "DamagePlayer" (/ 1.0 (`self.AttacksPerSecond`)) true))

(event `DamagePlayer`
  ;[1 1 1] Damage To Player
  (`/Game/Blueprints/BaseCharacter.AffectHealth` (`self.Player`) (`self.Damage`)))

(event `self.ReceiveActorEndOverlap`
  (params (OtherActor :type "Actor Object Reference"))
  ;[1 1 1] Damage To Player
  (if (== OtherActor (`self.Player`))
    (`KismetSystemLibrary.K2_ClearTimer` null "DamagePlayer")))

(event `OnCollideEvent`
  (params (EventName :type Name) (EmitterTime :type "Float (double-precision)") (ParticleTime :type Integer) (Location :type "Vector Structure") (Velocity :type "Vector Structure") (Direction :type "Vector Structure") (Normal :type "Vector Structure") (BoneName :type Name) (PhysMat :type "PhysicalMaterial Object Reference"))
  ;[1 1 1] Blood Splat
  (bind _returnvalue (`KismetMaterialLibrary.CreateDynamicMaterialInstance` "/Game/Blueprints/Blood_Splat/Splatter_Decal.Splatter_Decal"))
  (`MaterialInstanceDynamic.SetScalarParameterValue` _returnvalue "Frame" (`KismetMathLibrary.Conv_IntToDouble` (`KismetMathLibrary.RandomInteger` 11)))
  (`GameplayStatics.SpawnDecalAtLocation` _returnvalue (`KismetMathLibrary.Conv_DoubleToVector` (`KismetMathLibrary.RandomFloatInRange` 20.0 50.0)) Location (`KismetMathLibrary.Conv_VectorToRotator` (* Normal -1.0)) 20.0))

(fn `Calculate Death`
  (if (<= (`self.Health`) 0.0)
    (set `self.IsDead` true)
    (else
      (set `self.IsDead` false))))

(fn `Calculate Health`
  (params (Delta :type "Float (double-precision)"))
  (set `self.Health` (+ Delta (`self.Health`)))
  (`self.Calculate Death`))

(fn `UserConstructionScript`
  (bind _returnvalue (`PrimitiveComponent.CreateDynamicMaterialInstance` (`self.Mesh`) 0 null "None"))
  (bind _output_get (set `self.Mat` _returnvalue))
  (`MaterialInstanceDynamic.SetVectorParameterValue` _output_get "BodyColor" (`self.EnemyColour`)))