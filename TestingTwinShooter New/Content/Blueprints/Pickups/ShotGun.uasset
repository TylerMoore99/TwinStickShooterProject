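; Shotgun pickup actor that spins on a self-restarting Timeline, starts blinking after a delay, then destroys itself.
; When a BaseCharacter overlaps it, it replaces the character's current gun with a spawned shotgun attached to the gun socket.
; The pickup also plays a sound, updates the player's weapon HUD, sets weapon flags on the character and Save_Instance game instance, and removes its box and mesh.
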(event `ResetAnim`
  (bind (_direction _newtrack_0) (`Timeline|Timeline_0` :!via `PlayFromStart` :!label _label)
    (:`Update`
      (`SceneComponent.K2_SetWorldRotation` (`self.DefaultSceneRoot`) (`KismetMathLibrary.RLerp` (struct) (struct :`Yaw` 360.0) _newtrack_0) false false)
      (`KismetSystemLibrary.Delay` 10.0)
      (`KismetSystemLibrary.K2_SetTimerDelegate` (delegate `Flash`) 2.0 true)
      (`KismetSystemLibrary.Delay` 6.0)
      (`self.K2_DestroyActor`))
    (:`Finished`
      (`self.ResetAnim`))))

(event `self.ReceiveBeginPlay`
  (goto _label))

(event `Flash`
  (bind _staticmesh (`self.StaticMesh`))
  (`SceneComponent.SetVisibility` _staticmesh false false)
  (`KismetSystemLibrary.Delay` 1.0)
  (`SceneComponent.SetVisibility` _staticmesh true false))

(event `self.ReceiveActorBeginOverlap`
  (params (OtherActor :type "Actor Object Reference"))
  (bind _asbase_character (cast `/Game/Blueprints/BaseCharacter` OtherActor))
  (bind _assave_instance (cast `/Game/Blueprints/Save_Instance` (`GameplayStatics.GetGameInstance`)))
  (set `/Game/Blueprints/Save_Instance.Using Rifle Save` false _assave_instance)
  (`self.K2_DestroyActor` (`/Game/Blueprints/BaseCharacter.GunBase` _asbase_character))
  (bind _mesh (`Character.Mesh` _asbase_character))
  (bind _returnvalue (`|SpawnActorFromClass` "/Game/Blueprints/ShotGunWeapo.ShotGunWeapo_C" (`SceneComponent.K2_GetComponentToWorld` _mesh) "Undefined" "OverrideRootScale" null null))
  (bind _output_get (set `/Game/Blueprints/BaseCharacter.GunBase` _returnvalue _asbase_character))
  (`self.K2_AttachToComponent` _output_get _mesh "GunSocket" "SnapToTarget" "SnapToTarget" "SnapToTarget" true)
  (`GameplayStatics.PlaySound2D` "/Game/Sounds/GunPickup.GunPickup" 1.0 1.0 0.0 null null)
  (bind _asbase_character_2 (cast `/Game/Blueprints/BaseCharacter` (`GameplayStatics.GetPlayerCharacter` 0)))
  (`/Game/Blueprints/BaseCharacter.UpdateWeaponHUD` _asbase_character_2 2)
  (`ActorComponent.K2_DestroyComponent` (`self.Box`))
  (`ActorComponent.K2_DestroyComponent` (`self.StaticMesh`))
  (set `/Game/Blueprints/BaseCharacter.Using Rifle` true _asbase_character)
  (set `/Game/Blueprints/Save_Instance.Using Shotgun Save` true _assave_instance)
  (`KismetSystemLibrary.Delay` 120.0))

(fn `UserConstructionScript`)