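; A Freeze pickup that changes the walk speed of every Enemy when a BaseCharacter overlaps it.
; A looping timeline spins it and drives delays that start a visibility flash timer, then destroy the actor if those delays run out.
; On overlap it plays a sound and runs a second timeline whose Speed track sets each enemy's MaxWalkSpeed, while removing the pickup's box and mesh.
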(event `ResetAnim`
  (bind (_direction _newtrack_0) (`Timeline|Timeline_0` :!via `PlayFromStart` :!label _label)
    (:`Update`
      (`SceneComponent.K2_SetWorldRotation` (`self.DefaultSceneRoot`) (`KismetMathLibrary.RLerp` (struct) (struct :`Yaw` 360.0) _newtrack_0) false false)
      (`KismetSystemLibrary.Delay` 10.0)
      (`KismetSystemLibrary.K2_SetTimerDelegate` (delegate `Flash`) 2.0 true)
      (`KismetSystemLibrary.Delay` 6.0)
      (`self.K2_DestroyActor`))
    (:`Finished`
      (`self.ResetAnim`))))

(event `self.ReceiveBeginPlay`
  (goto _label))

(event `Flash`
  (bind _staticmesh (`self.StaticMesh`))
  (`SceneComponent.SetVisibility` _staticmesh false false)
  (`KismetSystemLibrary.Delay` 1.0)
  (`SceneComponent.SetVisibility` _staticmesh true false))

(event `self.ReceiveActorBeginOverlap`
  (params (OtherActor :type "Actor Object Reference"))
  (cast `/Game/Blueprints/BaseCharacter` OtherActor)
  (bind _outactors (`GameplayStatics.GetAllActorsOfClass` "/Game/Blueprints/Enemy.Enemy_C"))
  (`GameplayStatics.PlaySound2D` "/Game/Sounds/PowerUpCue.PowerUpCue" 1.0 1.0 0.0 null null)
  (bind (_direction _speed) (`Timeline|Timeline_1`)
    (:`Update`
      (for _array_element _outactors
        (set `CharacterMovementComponent.MaxWalkSpeed` _speed (`Character.CharacterMovement` _array_element))
        (`ActorComponent.K2_DestroyComponent` (`self.Box`))
        (`ActorComponent.K2_DestroyComponent` (`self.StaticMesh`))
        (`KismetSystemLibrary.Delay` 6.0)
        (`KismetSystemLibrary.PrintString` "Freeze")))))

(fn `UserConstructionScript`)