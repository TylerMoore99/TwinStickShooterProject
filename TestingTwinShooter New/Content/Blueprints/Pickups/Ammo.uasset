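; Ammo pickup actor that spins in place and replenishes a character's gun ammo on overlap.
; A timeline started at BeginPlay lerps the root's world rotation through a full turn, looping by restarting itself through ResetAnim when finished.
; Overlap by a BaseCharacter calls ReplenishAmmo on its GunBase, destroys the pickup, plays a 2D power-up sound and prints a debug message.
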(event `ResetAnim`
  (bind (_direction _newtrack_0) (`Timeline|Timeline_0` :!via `PlayFromStart` :!label _label)
    (:`Update`
      (`SceneComponent.K2_SetWorldRotation` (`self.DefaultSceneRoot`) (`KismetMathLibrary.RLerp` (struct) (struct :`Yaw` 360.0) _newtrack_0) false false))
    (:`Finished`
      (`self.ResetAnim`))))

(event `self.ReceiveBeginPlay`
  (goto _label))

(event `self.ReceiveActorBeginOverlap`
  (params (OtherActor :type "Actor Object Reference"))
  (bind _asbase_character (cast `/Game/Blueprints/BaseCharacter` OtherActor))
  (`/Game/Blueprints/GunBase.Replenish Ammo` (`/Game/Blueprints/BaseCharacter.GunBase` _asbase_character))
  (`self.K2_DestroyActor`)
  (`GameplayStatics.PlaySound2D` "/Game/Sounds/PowerUpCue.PowerUpCue" 1.0 1.0 0.0 null null)
  (`KismetSystemLibrary.PrintString` "Ammo"))

(fn `UserConstructionScript`)