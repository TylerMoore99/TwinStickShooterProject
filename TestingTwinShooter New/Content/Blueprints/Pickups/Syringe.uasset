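; Syringe speed-boost pickup that spins in the world until a BaseCharacter overlaps it.
; A timeline rotates the root through a full yaw turn and restarts itself on finish.
; On overlap, a second timeline's Speed curve drives the character's MaxWalkSpeed.
; Its update also removes the box and mesh, then destroys the actor after a delay and prints a debug message.
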(event `ResetAnim`
  (bind (_direction _newtrack_0) (`Timeline|Timeline_0` :!via `PlayFromStart` :!label _label)
    (:`Update`
      (`SceneComponent.K2_SetWorldRotation` (`self.DefaultSceneRoot`) (`KismetMathLibrary.RLerp` (struct) (struct :`Yaw` 360.0) _newtrack_0) false false))
    (:`Finished`
      (`self.ResetAnim`))))

(event `self.ReceiveBeginPlay`
  (goto _label))

(event `self.ReceiveActorBeginOverlap`
  (params (OtherActor :type "Actor Object Reference"))
  (bind _asbase_character (cast `/Game/Blueprints/BaseCharacter` OtherActor))
  (bind (_direction _speed) (`Timeline|Timeline_1`)
    (:`Update`
      (set `CharacterMovementComponent.MaxWalkSpeed` _speed (`Character.CharacterMovement` _asbase_character))
      (`ActorComponent.K2_DestroyComponent` (`self.Box`))
      (`ActorComponent.K2_DestroyComponent` (`self.StaticMesh`))
      (`KismetSystemLibrary.Delay` 6.0)
      (`self.K2_DestroyActor`)
      (`KismetSystemLibrary.PrintString` "Boost"))))

(fn `UserConstructionScript`)