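; Rifle pickup that spins on a looping timeline and arms any BaseCharacter that overlaps it.
; On overlap it destroys the character's current GunBase, spawns a Rifle2 as the replacement and attaches it to the mesh's GunSocket.
; It then plays a sound, updates player 0's weapon HUD, sets rifle flags on the character and Save_Instance game instance, and destroys itself.
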(event `ResetAnim`
  (bind (_direction _newtrack_0) (`Timeline|Timeline_0` :!via `PlayFromStart` :!label _label)
    (:`Update`
      (`SceneComponent.K2_SetWorldRotation` (`self.DefaultSceneRoot`) (`KismetMathLibrary.RLerp` (struct) (struct :`Yaw` 360.0) _newtrack_0) false false))
    (:`Finished`
      (`self.ResetAnim`))))

(event `self.ReceiveBeginPlay`
  (goto _label))

(event `self.ReceiveActorBeginOverlap`
  (params (OtherActor :type "Actor Object Reference"))
  (bind _asbase_character (cast `/Game/Blueprints/BaseCharacter` OtherActor))
  (`self.K2_DestroyActor` (`/Game/Blueprints/BaseCharacter.GunBase` _asbase_character))
  (bind _mesh (`Character.Mesh` _asbase_character))
  (bind _returnvalue (`|SpawnActorFromClass` "/Game/Blueprints/Rifle-2.Rifle-2_C" (`SceneComponent.K2_GetComponentToWorld` _mesh) "Undefined" "OverrideRootScale" null null))
  (bind _output_get (set `/Game/Blueprints/BaseCharacter.GunBase` _returnvalue _asbase_character))
  (`self.K2_AttachToComponent` _output_get _mesh "GunSocket" "SnapToTarget" "SnapToTarget" "SnapToTarget" true)
  (`GameplayStatics.PlaySound2D` "/Game/Sounds/GunPickup.GunPickup" 1.0 1.0 0.0 null null)
  (bind _asbase_character_2 (cast `/Game/Blueprints/BaseCharacter` (`GameplayStatics.GetPlayerCharacter` 0)))
  (`/Game/Blueprints/BaseCharacter.UpdateWeaponHUD` _asbase_character_2 1)
  (set `/Game/Blueprints/BaseCharacter.Using Rifle` true _asbase_character)
  (bind _assave_instance (cast `/Game/Blueprints/Save_Instance` (`GameplayStatics.GetGameInstance`)))
  (set `/Game/Blueprints/Save_Instance.Using Rifle Save` true _assave_instance)
  (`self.K2_DestroyActor`))

(fn `UserConstructionScript`)