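; Shotgun weapon Blueprint that spawns projectiles and manages magazine and reserve ammo.
; Trigger pull fires once and starts a looping timer at the fire rate, cleared on release.
; Each shot waits on a Delay, then spawns one projectile or auto-reloads when empty.
; A delayed, flag-guarded reload refills the magazine from reserve, and a replenish event restores the reserve to maximum.
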(event `CustomEvent`
  ;[1 1 1] Trigger Pull
  (`/Engine/EditorBlueprintResources/StandardMacros.DoOnce` false :!label _label
    (:`Completed`
      (`self.Fire`)
      (`KismetSystemLibrary.K2_SetTimer` null "Fire" (/ 1.0 (`self.Rounds Per Second`)) true))))

(event `CustomEvent_1`
  ;[1 1 1] Trigger Pull
  (`KismetSystemLibrary.K2_ClearTimer` null "Fire")
  (goto _label :!via `Reset`))

(event `CustomEvent_2`
  ;[1 1 1] Firing Bullets
  (set `self.Will Fire` false)
  (`KismetSystemLibrary.Delay` 2.0)
  (set `self.Will Fire` true)
  (if (<= (`self.Ammo`) 0)
    (if (== (`self.ReserveAmmo`) 0)
      _
      (elif (not (`self.ReloadInternal`))
        (set `self.ReloadInternal` true)
        (`self.Event_reloadInternal`)))
    (else
      (set `self.Ammo` (- (`self.Ammo`) 1))
      (set `self.ReloadInternal` false)
      (`|SpawnActorFromClass` (`self.Projectile`) (`SceneComponent.K2_GetComponentToWorld` (`self.ProjectilerSpawnPoint`)) "Undefined" "OverrideRootScale" null null))))

(event `CustomEvent_3`
  ;[1 1 1] Reload
  (if (not (`self.ReloadInternal`))
    (set `self.ReloadInternal` true)
    (`self.Event_reloadInternal`)))

(event `CustomEvent_4`
  (bind _magsize (`self.MagSize`))
  ;[1 1 1] Reload
  (`KismetSystemLibrary.Delay` 2.0)
  (if (`self.ReloadInternal`)
    (if (< (- (`self.ReserveAmmo`) (`self.MagSize`)) 0)
      (set `self.Ammo` (`self.ReserveAmmo`))
      (set `self.ReserveAmmo` 0)
      (else
        (set `self.Ammo` _magsize)
        (set `self.ReserveAmmo` (- (`self.ReserveAmmo`) _magsize))))
    (set `self.ReloadInternal` false)))

(event `CustomEvent_5`
  ;[1 1 1] Replenish Ammo
  (set `self.ReserveAmmo` (`self.Maximum Ammo`))
  (if (<= (`self.ReserveAmmo`) 0)
    (if (<= (`self.Ammo`) 0)
      (`self.Event_reloadInternal`))))

(fn `UserConstructionScript`
  (`parent.UserConstructionScript`))