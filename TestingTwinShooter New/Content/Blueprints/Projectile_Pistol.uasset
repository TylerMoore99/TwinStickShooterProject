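; Pistol projectile actor that deals damage on overlap and plays an attached firing sound when spawned.
; Overlapping an IDamageable actor not tagged Friendly sends damage through the interface and spawns a floating damage-number widget at the projected screen position.
; Those hits and overlaps with non-damageable actors play a splat sound and destroy the projectile, while Friendly damageable actors are ignored.
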(event `self.ReceiveBeginPlay`
  (`GameplayStatics.SpawnSoundAttached` "/Game/Sounds/Pistol_-_Sound_Effect.Pistol_-_Sound_Effect" (`self.BulletMesh`) "None" (0.0 0.0 0.0) (struct) "KeepRelativeOffset" false 1.0 1.0 0.0 null null))

(event `self.ReceiveActorBeginOverlap`
  (params (OtherActor :type "Actor Object Reference"))
  (if (`KismetSystemLibrary.DoesImplementInterface` OtherActor "/Game/Blueprints/IDamageable.IDamageable_C")
    (if (not (`self.ActorHasTag` OtherActor "Friendly"))
      (message `/Game/Blueprints/IDamageable.AffectHealth` OtherActor (`self.Damage`))
      (`self.FloatingNumbersPistol` (`self.K2_GetActorLocation`) (`self.PistolDamage`))
      (`GameplayStatics.SpawnSoundAttached` "/Game/Sounds/Splat_Sound_Effect.Splat_Sound_Effect" (`self.ProjectileCollision`) "None" (0.0 0.0 0.0) (struct) "KeepRelativeOffset" false 1.0 1.0 0.0 null null :!label _label)
      (`self.K2_DestroyActor`))
    (else
      (goto _label))))

(fn `FloatingNumbersPistol`
  (params (Location :type "Vector Structure") (Damage :type "Float (double-precision)"))
  (bind _returnvalue (`|CreateWidget` "/Game/UI/DamageNumbers.DamageNumbers_C" null Damage (`GameplayStatics.ProjectWorldToScreen` (`GameplayStatics.GetPlayerController` 0) Location)))
  (`UserWidget.AddToViewport` _returnvalue 0))

(fn `UserConstructionScript`
  (`parent.UserConstructionScript`))