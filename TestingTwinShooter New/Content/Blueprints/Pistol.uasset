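; Pistol weapon Blueprint with automatic fire, a magazine and reserve ammo.
; A DoOnce-gated start event fires if ammo remains and loops a Fire timer at the rounds-per-second rate; a stop event clears both.
; Each shot decrements ammo, then spawns a projectile and attached sound.
; At zero it skips the shot and, given reserve, refills after a delay, deducting a fixed amount rather than MagSize.
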(event `CustomEvent`
  (`/Engine/EditorBlueprintResources/StandardMacros.DoOnce` false :!label _label
    (:`Completed`
      (if (not (== (`self.Ammo`) 0))
        (`self.Fire`)
        (`KismetSystemLibrary.K2_SetTimer` null "Fire" (/ 1.0 (`self.Rounds Per Second`)) true)))))

(event `CustomEvent_1`
  (`KismetSystemLibrary.K2_ClearTimer` null "Fire")
  (goto _label :!via `Reset`))

(event `CustomEvent_2`
  ;[1 1 1] Firing Bullets
  (set `self.Ammo` (- (`self.Ammo`) 1))
  (if (== (`self.Ammo`) 0)
    (if (not (== (`self.ReserveAmmo`) 0))
      (`KismetSystemLibrary.Delay` 2.0)
      (set `self.Ammo` (`self.MagSize`))
      (set `self.ReserveAmmo` (- (`self.ReserveAmmo`) 30)))
    (else
      (`|SpawnActorFromClass` "/Game/Blueprints/Projectile_Pistol.Projectile_Pistol_C" (`SceneComponent.K2_GetComponentToWorld` (`self.ProjectilerSpawnPoint`)) "Undefined" "OverrideRootScale" null null)
      (`GameplayStatics.SpawnSoundAttached` "/Game/Sounds/Pistol_-_Sound_Effect.Pistol_-_Sound_Effect" (`self.GunMesh`) "None" (0.0 0.0 0.0) (struct) "KeepRelativeOffset" false 1.0 1.0 0.0 null null))))

(fn `UserConstructionScript`
  (`parent.UserConstructionScript`))