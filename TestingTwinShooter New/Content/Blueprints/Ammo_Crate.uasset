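; Ammo crate actor that sells an ammo refill for points in a twin-stick game.
; Overlapping its collision with a BaseCharacter shows a text prompt and opens a Gate, while leaving hides and closes it.
; With the gate open, the gamepad right face button checks the TwinStickMode score, then replenishes the player's gun, deducts the fixed cost and plays a sound.
; The crate enables its own input on BeginPlay to receive that button directly.
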(event `self.ReceiveBeginPlay`
  (`self.EnableInput` (`GameplayStatics.GetPlayerController` 0)))

(event `Key|Gamepad_FaceButton_Right`
  (params (Key :type "Key Structure"))
  (:`Pressed`
    (`/Engine/EditorBlueprintResources/StandardMacros.Gate` true :!label _label
      (:`Exit`
        (bind _astwin_stick_mode (cast `/Game/Blueprints/TwinStickMode` (`GameplayStatics.GetGameMode`)))
        (bind _score (`/Game/Blueprints/TwinStickMode.Score` _astwin_stick_mode))
        (if (>= _score 750)
          (bind _asbase_character (cast `/Game/Blueprints/BaseCharacter` (`GameplayStatics.GetPlayerCharacter` 0)))
          (`/Game/Blueprints/GunBase.Replenish Ammo` (`/Game/Blueprints/BaseCharacter.GunBase` _asbase_character))
          (set `/Game/Blueprints/TwinStickMode.Score` (- _score 750) _astwin_stick_mode)
          (`GameplayStatics.PlaySound2D` "/Game/Sounds/PointsSpent.PointsSpent" 1.0 1.0 0.0 null null))))))

(event `self.Collsions.OnComponentBeginOverlap`
  (params (OverlappedComponent :type "PrimitiveComponent Object Reference") (OtherActor :type "Actor Object Reference") (OtherComp :type "PrimitiveComponent Object Reference") (OtherBodyIndex :type Integer) (bFromSweep :type Boolean) (SweepResult :type "HitResult Structure (by ref)"))
  (cast `/Game/Blueprints/BaseCharacter` OtherActor)
  (`SceneComponent.SetVisibility` (`self.Writing`) true false)
  (goto _label :!via `Open`))

(event `self.Collsions.OnComponentEndOverlap`
  (params (OverlappedComponent :type "PrimitiveComponent Object Reference") (OtherActor :type "Actor Object Reference") (OtherComp :type "PrimitiveComponent Object Reference") (OtherBodyIndex :type Integer))
  (cast `/Game/Blueprints/BaseCharacter` OtherActor)
  (`SceneComponent.SetVisibility` (`self.Writing`) false false)
  (goto _label :!via `Close`))

(fn `UserConstructionScript`)