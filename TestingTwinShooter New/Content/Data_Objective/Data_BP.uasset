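; Data_BP is an interactable pickup actor, in the Data_Objective folder, that the player removes from the level with the F key.
; It enables input for the first player controller on BeginPlay, and F destroys the actor if the player's BaseCharacter overlaps its Box.
; Any begin or end overlap on the Box toggles the PickUp component's visibility, with no check on which actor overlaps.
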(event `self.ReceiveBeginPlay`
  (`self.EnableInput` (`GameplayStatics.GetPlayerController` 0)))

(event `Key|F` :consume false
  (params (Key :type "Key Structure"))
  (:`Pressed`
    (bind _asbase_character (cast `/Game/Blueprints/BaseCharacter` (`GameplayStatics.GetPlayerCharacter` 0)))
    (if (`PrimitiveComponent.IsOverlappingActor` (`self.Box`) _asbase_character)
      (`self.K2_DestroyActor`))))

(event `self.Box.OnComponentBeginOverlap`
  (params (OverlappedComponent :type "PrimitiveComponent Object Reference") (OtherActor :type "Actor Object Reference") (OtherComp :type "PrimitiveComponent Object Reference") (OtherBodyIndex :type Integer) (bFromSweep :type Boolean) (SweepResult :type "HitResult Structure (by ref)"))
  (`SceneComponent.ToggleVisibility` (`self.Pick Up`) false))

(event `self.Box.OnComponentEndOverlap`
  (params (OverlappedComponent :type "PrimitiveComponent Object Reference") (OtherActor :type "Actor Object Reference") (OtherComp :type "PrimitiveComponent Object Reference") (OtherBodyIndex :type Integer))
  (`SceneComponent.ToggleVisibility` (`self.Pick Up`) false))

(fn `UserConstructionScript`)