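; Player character Blueprint for a twin-stick shooter, handling movement, aim-to-fire, health and respawn.
; On BeginPlay it spawns a Pistol on the mesh's GunSocket, caches TwinStickMode and creates the HUD.
; Move axes drive world-space movement; look axes share logic that sets control rotation and holds the trigger beyond a deadzone.
; AffectHealth updates health; on death it disables input, waits, requests a GameMode respawn, then destroys pistol and character.
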(event `InputAxis|MoveUp`
  (params (AxisValue :type "Float (single-precision)"))
  ;[1 1 1] Movement
  (`self.AddMovementInput` (1.0 0.0 0.0) AxisValue))

(event `InputAxis|LookUp`
  (params (AxisValue :type "Float (single-precision)"))
  (bind _pistol (`self.Pistol`))
  ;[1 1 1] Rotation
  (bind _returnvalue (`KismetMathLibrary.MakeVector` AxisValue (stale `InputAxis|LookRight` AxisValue)))
  (if (> (`KismetMathLibrary.VSize` _returnvalue) 0.25) :!label _label
    (`Controller.SetControlRotation` (`self.GetController`) (`KismetMathLibrary.Conv_VectorToRotator` _returnvalue))
    (`/Game/Blueprints/Pistol.PullTrigger` _pistol)
    (else
      (`/Game/Blueprints/Pistol.ReleaseTrigger` _pistol))))

(event `InputAxis|LookRight`
  (params (AxisValue :type "Float (single-precision)"))
  ;[1 1 1] Rotation
  (goto _label))

(event `InputAxis|MoveRight`
  (params (AxisValue :type "Float (single-precision)"))
  ;[1 1 1] Movement
  (`self.AddMovementInput` (0.0 1.0 0.0) AxisValue))

(event `/Game/Blueprints/IDamageable.AffectHealth`
  (params (Delta :type "Float (single-precision)"))
  ;[1 1 1] Destroys Player And Weapon
  (`self.CalculateHealth` Delta)
  (`KismetSystemLibrary.PrintString` (`KismetStringLibrary.Conv_DoubleToString` (`self.Health`)))
  (if (`self.IsDead`)
    (`self.DisableInput` null)
    (`KismetSystemLibrary.Delay` 3.0)
    (`/Game/Blueprints/TwinStickMode.RespawnPlayer` (`self.GameMode`))
    (`self.K2_DestroyActor` (`self.Pistol`))
    (`self.K2_DestroyActor` self)))

(event `self.ReceiveBeginPlay`
  (bind _mesh (`self.Mesh`))
  ;[1 1 1] Weapon Selection & Respawn
  (`|ExecutionSequence`
    (:`then_0`
      (bind _returnvalue (`|SpawnActorFromClass` "/Game/Blueprints/Pistol.Pistol_C" (`SceneComponent.K2_GetComponentToWorld` _mesh) "Undefined" "OverrideRootScale" null null))
      (bind _output_get (set `self.Pistol` _returnvalue))
      (`self.K2_AttachToComponent` _output_get _mesh "GunSocket" "KeepWorld" "KeepRelative" "KeepRelative" true))
    (:`then_1`
      (bind _astwin_stick_mode (cast `/Game/Blueprints/TwinStickMode` (`GameplayStatics.GetGameMode`)))
      (bind _output_get_2 (set `self.GameMode` _astwin_stick_mode)))
    (:`then_2`
      (bind _returnvalue_2 (`|CreateWidget` "/Game/Blueprints/TwinStickHUD.TwinStickHUD_C"))
      (`UserWidget.AddToViewport` _returnvalue_2 0))))

(fn `CalculateDead`
  (if (<= (`self.Health`) 0.0)
    (set `self.IsDead` true)
    (else
      (set `self.IsDead` false))))

(fn `CalculateHealth`
  (params (Delta :type "Float (double-precision)"))
  (set `self.Health` (+ Delta (`self.Health`)))
  (`self.CalculateDead`))

(fn `UserConstructionScript`)