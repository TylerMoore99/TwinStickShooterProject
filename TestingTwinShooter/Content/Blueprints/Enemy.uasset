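; Enemy character for a twin-stick game that damages overlapping player characters and awards kills and score when killed.
; Overlapping a BaseCharacter starts a looping DamagePlayer timer at the attack rate, cleared when that player leaves.
; AffectHealth adds a signed delta; death detaches the controller, removes damage volume and some collision, updates TwinStickMode, then destroys the actor after a delay.
; The construction script tints the body through a dynamic material.
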(event `/Game/Blueprints/IDamageable.AffectHealth`
  (params (Delta :type "Float (single-precision)"))
  (bind _capsulecomponent (`self.CapsuleComponent`))
  ;[1 1 1] Damage To Enemy & Value of Score
  (`self.Calculate Health` Delta)
  (`KismetSystemLibrary.PrintString` (`KismetStringLibrary.Conv_DoubleToString` (`self.Health`)))
  (if (`self.IsDead`)
    (`self.DetachFromControllerPendingDestroy`)
    (`ActorComponent.K2_DestroyComponent` (`self.DamageVolume`))
    (`PrimitiveComponent.SetCollisionResponseToChannel` _capsulecomponent "ECC_WorldDynamic" "ECR_Ignore")
    (`PrimitiveComponent.SetCollisionResponseToChannel` _capsulecomponent "ECC_Pawn" "ECR_Ignore")
    (bind _astwin_stick_mode (cast `/Game/Blueprints/TwinStickMode` (`GameplayStatics.GetGameMode`)))
    (`/Game/Blueprints/TwinStickMode.IncrementKills` _astwin_stick_mode 1)
    (`/Game/Blueprints/TwinStickMode.IncrementScore` _astwin_stick_mode 100)
    (`KismetSystemLibrary.Delay` 15.0)
    (`self.K2_DestroyActor`)))

(event `self.ReceiveActorBeginOverlap`
  (params (OtherActor :type "Actor Object Reference"))
  ;[1 1 1] Damage To Player
  (bind _asbase_character (cast `/Game/Blueprints/BaseCharacter` OtherActor))
  (set `self.Player` _asbase_character)
  (`KismetSystemLibrary.K2_SetTimer` null "DamagePlayer" (/ 1.0 (`self.AttacksPerSecond`)) true))

(event `DamagePlayer`
  ;[1 1 1] Damage To Player
  (`/Game/Blueprints/BaseCharacter.AffectHealth` (`self.Player`) (`self.Damage`)))

(event `self.ReceiveActorEndOverlap`
  (params (OtherActor :type "Actor Object Reference"))
  ;[1 1 1] Damage To Player
  (if (== OtherActor (`self.Player`))
    (`KismetSystemLibrary.K2_ClearTimer` null "DamagePlayer")))

(fn `Calculate Death`
  (if (<= (`self.Health`) 0.0)
    (set `self.IsDead` true)
    (else
      (set `self.IsDead` false))))

(fn `Calculate Health`
  (params (Delta :type "Float (double-precision)"))
  (set `self.Health` (+ Delta (`self.Health`)))
  (`self.Calculate Death`))

(fn `UserConstructionScript`
  (bind _returnvalue (`PrimitiveComponent.CreateDynamicMaterialInstance` (`self.Mesh`) 0 null))
  (bind _output_get (set `self.Mat` _returnvalue))
  (`MaterialInstanceDynamic.SetVectorParameterValue` _output_get "BodyColor" (`self.EnemyColour`)))